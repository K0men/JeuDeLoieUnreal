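; Board actor for a dice board game that moves the player character along a looping array of tiles.
; Pressing R rolls a six-sided die, locked while busy, and StepForward recursively moves the capsule tile by tile at constant speed, facing each target.
; On arrival, the tile's offset triggers one bonus or malus move forward or backward after a pause, without chaining.
; BeginPlay disables character movement and snaps the player to the first tile.
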(event Custom|RollDice
  (if (not (Variables|Default|GetIsBusy))
    (Variables|Default|SetIsBusy true)
    (Variables|Default|SetOffsetApplied false)
    (Variables|Default|SetDiceResult (Math|Random|RandomIntegerinRange 1 6))
    (Development|PrintString (Utilities|String|ToString(Integer) (Variables|Default|GetDiceResult)))
    (CallFunction|StepForward (Variables|Default|GetDiceResult) 1)))

(event Custom|StepForward
  (params (Remaining :type Integer) (Dir :type Integer))
  (bind _tiles (Variables|Default|GetTiles))
  (bind _returnvalue (Utilities|Array|Length _tiles))
  (if (> Remaining 0)
    (bind _output_get (Variables|Default|SetCurrent%20Index (Math|Integer|%(Integer) (+ (Variables|Default|GetCurrent%20Index) Dir _returnvalue) _returnvalue)))
    (Variables|Default|SetTargetLocation (+ (Transformation|GetActorLocation (Utilities|Array|Get(acopy) (Variables|Default|GetTiles) _output_get)) (Math|Vector|MakeVector 0.0 0.0 (Variables|Default|GetHeightOffset))))
    (Components|MoveComponentTo (Variables|/Script/Engine.Character|GetCapsuleComponent (Variables|Default|GetPlayerRef)) (Variables|Default|GetTargetLocation) (Math|Rotator|MakeRotator 0.0 0.0 (.Yaw (Math|Rotator|BreakRotator (Math|Rotator|FindLookatRotation (Transformation|GetActorLocation (Variables|Default|GetPlayerRef)) (Variables|Default|GetTargetLocation))))) false false (/ (Math|Vector|Distance(Vector) (Transformation|GetActorLocation (Variables|Default|GetPlayerRef)) (Variables|Default|GetTargetLocation)) (Variables|Default|GetMoveSpeed)) false)
    (CallFunction|StepForward (- Remaining 1) Dir)
    (else
      ;[0.15 0.15 0.15 0.5] Plus de cases donc on avance plus.
      (CallFunction|OnArrived))))

(event Custom|OnArrived
  (bind _offset (Default|GetOffSet (Utilities|Array|Get(acopy) (Variables|Default|GetTiles) (Variables|Default|GetCurrent%20Index))))
  (Variables|Default|SetOffset _offset)
  (if (and (!= (Variables|Default|GetOffset) 0) (not (Variables|Default|GetOffsetApplied)))
    (Variables|Default|SetOffsetApplied true)
    (if (> (Variables|Default|GetOffset) 0)
      (Development|PrintString (Utilities|String|Append "Bonus ! " (Utilities|String|ToString(Integer) (Variables|Default|GetOffset))))
      (else
        (Development|PrintString (Utilities|String|Append "Malus ! " (Utilities|String|ToString(Integer) (Math|Integer|Absolute(Integer) (Variables|Default|GetOffset)))))))
    (Utilities|FlowControl|Delay (Variables|Default|GetPauseTime))
    (CallFunction|StepForward (Math|Integer|Absolute(Integer) (Variables|Default|GetOffset)) (Class|KismetMathLibrary|SignOfInteger (Variables|Default|GetOffset)))
    (else
      (Variables|Default|SetIsBusy false))))

(event EventBeginPlay
  (Variables|Default|SetPlayerRef (Game|GetPlayerCharacter 0))
  (Pawn|Components|CharacterMovement|DisableMovement (Variables|/Script/Engine.Character|GetCharacterMovement (Variables|Default|GetPlayerRef)))
  (Transformation|SetActorLocation (Variables|Default|GetPlayerRef) (+ (Transformation|GetActorLocation (Utilities|Array|Get(acopy) (Variables|Default|GetTiles))) (Math|Vector|MakeVector 0.0 0.0 (Variables|Default|GetHeightOffset))) false false)
  (bind _output_get (Variables|Default|SetCurrent%20Index 0))
  (Input|EnableInput (Game|GetPlayerController _output_get)))

(event Input|KeyboardEvents|R
  (params (Key :type Key%20Structure :default "None"))
  (:Pressed
    (CallFunction|RollDice)))

(fn ConstructionScript)