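; Board Blueprint for a tile-based dice game that places the player character at the start of the board.
; On BeginPlay it disables character movement, moves the player to the first entry in Tiles plus a height offset, resets the current index and enables input.
; RollDice only sets the busy flag and clears OffsetApplied; the random 1–6 roll is unconnected and no tile-to-tile movement is present.
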(event Custom|RollDice
  (if (not (Variables|Default|GetIsBusy))
    (Variables|Default|SetIsBusy true)
    (Variables|Default|SetOffsetApplied false)))

(event EventBeginPlay
  (Variables|Default|SetPlayerRef (Game|GetPlayerCharacter 0))
  (Pawn|Components|CharacterMovement|DisableMovement (Variables|/Script/Engine.Character|GetCharacterMovement (Variables|Default|GetPlayerRef)))
  (Transformation|SetActorLocation (Variables|Default|GetPlayerRef) (+ (Transformation|GetActorLocation (Utilities|Array|Get(acopy) (Variables|Default|GetTiles))) (Math|Vector|MakeVector 0.0 0.0 (Variables|Default|GetHeightOffset))) false false)
  (bind _output_get (Variables|Default|SetCurrent%20Index 0))
  (Input|EnableInput (Game|GetPlayerController _output_get) 0))

(fn ConstructionScript)